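; Door actor that the player opens and closes with E while its trigger box is overlapped, provided they hold a key.
; Trigger overlap enables and disables input on the door itself for player controller 0.
; Pressing E checks Key1 on MyCharacter, printing a hint if it is missing, otherwise flipping DoorStatus to play or reverse the DoorRotation timeline.
; The timeline drives the whole actor's relative yaw.
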(event `self.TriggerBox.OnComponentBeginOverlap`
  (params (OtherActor :type "Actor Object Reference") (OtherComp :type "PrimitiveComponent Object Reference") (OtherBodyIndex :type Integer) (bFromSweep :type Boolean) (SweepResult :type "EngineTypes.HitResult Structure (by ref)"))
  (`self.EnableInput` (`GameplayStatics.GetPlayerController` 0)))

(event `Key|E`
  (:`Pressed`
    (bind _asmycharacter_c (cast `/Game/Blueprints/MyCharacter` (`GameplayStatics.GetPlayerCharacter` 0)))
    (if (`/Game/Blueprints/MyCharacter.Key1` _asmycharacter_c)
      (if (`self.DoorStatus`)
        (set `self.DoorStatus` false)
        (bind (_direction _doorrot) (`Timeline|DoorRotation` :!label _label)
          (:`Update`
            (`self.SetActorRelativeRotation` (`KismetMathLibrary.MakeRot` 0.0 _doorrot))))
        (else
          (set `self.DoorStatus` true)
          (goto _label :!via `Reverse`)))
      (else
        (`KismetSystemLibrary.PrintString` "You need the key!")))))

(event `self.TriggerBox.OnComponentEndOverlap`
  (params (OtherActor :type "Actor Object Reference") (OtherComp :type "PrimitiveComponent Object Reference") (OtherBodyIndex :type Integer))
  (`self.DisableInput` (`GameplayStatics.GetPlayerController` 0)))

(fn `UserConstructionScript`)